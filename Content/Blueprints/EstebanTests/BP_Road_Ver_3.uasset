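; Unfinished test Blueprint for a spline road actor, meant to build spline meshes from a right spline and averaged edge data.
; Its construction script calls SetMeshAtSplineIndex in a loop whose count input is unset, so it never iterates.
; That function only computes LOD-subdivided segment times along SplineRight.
; Mesh creation, width scaling, roll, up-vector and debug arrow code is disconnected, as are the initialization calls.
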(event EventBeginPlay)

(event Collision|EventActorBeginOverlap
  (params (OtherActor :type Actor%20Object%20Reference)))

(event EventTick
  (params (DeltaSeconds :type Float%20%28single-precision%29)))

(fn ConstructionScript
  (for _index (range 0 (- 0 2))
    (CallFunction|SetMeshatSplineIndex _index)))

(fn DrawDebug
  ;[1 1 1] Comment
  (for _index (range 0 (- (Spline|GetNumberOfSplinePoints (Variables|Default|GetSplineRight)) 1))
    _))

(fn InitializeArrays
  (Utilities|Array|Resize (Variables|Default|GetmeshList) (- 0 1)))

(fn InitializeSplines)

(fn SetMeshatSplineIndex
  (params (Index :type Integer))
  (bind _lod (Variables|Default|GetLOD))
  (bind _lod_2 (Variables|Default|GetLOD))
  (bind _splineright (Variables|Default|GetSplineRight))
  (bind _returnvalue (Math|Conversions|ToFloat(Integer) _lod))
  (bind _returnvalue_2 (Math|Conversions|ToFloat(Integer) _lod_2))
  (LocalVariables|SetRightTimeStart (Class|SplineComponent|GetTimeatDistanceAlongSpline _splineright (Spline|GetDistanceAlongSplineatSplinePoint _splineright Index)))
  (LocalVariables|SetRightTimeEnd (Class|SplineComponent|GetTimeatDistanceAlongSpline _splineright (Spline|GetDistanceAlongSplineatSplinePoint _splineright (+ Index 1))))
  (for _index (range 1 (Variables|Default|GetLOD))
    ;[1 1 1] Set Right Segment Start Time
    (LocalVariables|SetRightSegmentTimeStart (Math|Float|Lerp (LocalVariables|GetRightTimeStart) (LocalVariables|GetRightTimeEnd) (- (/ (Math|Conversions|ToFloat(Integer) _index) _returnvalue_2) (/ 1.0 _returnvalue_2))))
    ;[1 1 1] Set Right Segment End Time
    (LocalVariables|SetRightSegmentTimeEnd (Math|Float|Lerp (LocalVariables|GetRightTimeStart) (LocalVariables|GetRightTimeEnd) (- (/ (Math|Conversions|ToFloat(Integer) (+ _index 1)) _returnvalue) (/ 1.0 _returnvalue))))))

(fn Midpoint
  (params (Vector1 :type Vector) (Vector2 :type Vector))
  (return (/ (+ Vector1 Vector2) 2)))