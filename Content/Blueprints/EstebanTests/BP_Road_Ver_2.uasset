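; Road builder actor that generates spline meshes in its construction script from separate left and right edge splines.
; Each span between point pairs is split into LOD segments, positioned on the right spline with tangents averaged from both edges.
; Distance between edges drives width scale, and rotated cross-edge vectors set up direction, allowing banking.
; Debug arrows are added; computed rolls and point add/delete detection are left unused.
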(event EventBeginPlay)

(event Collision|EventActorBeginOverlap
  (params (OtherActor :type Actor%20Object%20Reference)))

(event EventTick
  (params (DeltaSeconds :type Float%20%28single-precision%29)))

(fn ConstructionScript
  ;[1 1 1] Initialization
  (CallFunction|InitializeSplines)
  (CallFunction|InitializeArrays)
  (CallFunction|DrawDebug)
  (for _index (range 0 (- (Variables|Default|GetminPoints) 2))
    (CallFunction|SetMeshatSplineIndex _index)))

(fn DrawDebug
  (bind _splineright (Variables|Default|GetSplineRight))
  (bind _returnvalue (Spline|GetNumberOfSplinePoints _splineright))
  (bind _returnvalue_2 (- _returnvalue 1))
  ;[1 1 1] Comment
  (for _index (range 0 _returnvalue_2)
    _)
  ;[1 1 1] Comment
  (for _index_2 (range 0 (- _returnvalue_2 1)) ; Iterate through each mesh index
    (bind _newparam (CallFunction|GetMidpointatIndex (+ _index_2 1)))
    (bind _newparam_2 (CallFunction|GetMidpointatIndex _index_2))
    (bind _midpoint (CallFunction|Midpoint _newparam_2 _newparam))
    (bind _up_vector (CallFunction|GetUpatMeshIndex _index_2))
    (AddComponent|AddArrowComponent false (Math|Transform|MakeTransform _midpoint (Math|Conversions|RotationFromXVector _up_vector) "1.000000,1.000000,1.000000"))))

(fn InitializeArrays
  (bind _minpoints (Variables|Default|GetminPoints))
  (bind _rolllist (Variables|Default|GetrollList))
  (bind _rolllist_2 (Variables|Default|GetrollList))
  (bind _returnvalue (- _minpoints 1))
  (Utilities|Array|Resize (Variables|Default|GetmeshList) _returnvalue)
  (Utilities|Array|Resize _rolllist _minpoints)
  (Utilities|Array|SetArrayElem _rolllist 0 0.0)
  (for _index (range 1 _returnvalue)
    (bind _up_vector (CallFunction|GetUpatSplineIndex _index))
    (bind _right_axis (CallFunction|CalculateRightatIndex _index))
    (bind _forward_vector (CallFunction|GetForwardatIndex _index))
    (Utilities|Array|SetArrayElem _rolllist_2 _index (+ (Math|Trig|DegreesToRadians (Math|Float|ClampAngle (Math|Trig|RadiansToDegrees (- (- (* (Math|Trig|DegreesToRadians (.roll (Math|Rotator|MakeRotationfromAxes _forward_vector _right_axis _up_vector))) -1.0) 3.14) (Utilities|Array|Get(acopy) _rolllist_2 (- _index 1)))) -9e+01 9e+01)) (Utilities|Array|Get(acopy) _rolllist_2 (- _index 1))))))

(fn InitializeSplines
  (bind _output_get (Variables|Default|SetminPoints (Math|Integer|Min(Integer) (Spline|GetNumberOfSplinePoints (Variables|Default|GetSplineRight)) (Spline|GetNumberOfSplinePoints (Variables|Default|GetSplineLeft)))))
  (for _index (range 0 (- _output_get 1))
    _))

(fn SetMeshatSplineIndex
  (params (Index :type Integer))
  (bind _lod (Variables|Default|GetLOD))
  (bind _lod_2 (Variables|Default|GetLOD))
  (bind _splineright (Variables|Default|GetSplineRight))
  (bind _lod_3 (Variables|Default|GetLOD))
  (bind _splineleft (Variables|Default|GetSplineLeft))
  (bind _lod_4 (Variables|Default|GetLOD))
  (bind _splineright_2 (Variables|Default|GetSplineRight))
  (bind _splineleft_2 (Variables|Default|GetSplineLeft))
  (bind _splineleft_3 (Variables|Default|GetSplineLeft))
  (bind _splineright_3 (Variables|Default|GetSplineRight))
  (bind _returnvalue (Math|Conversions|ToFloat(Integer) _lod))
  (bind _returnvalue_2 (Math|Conversions|ToFloat(Integer) _lod_2))
  (bind _returnvalue_3 (Math|Conversions|ToFloat(Integer) _lod_3))
  (bind _returnvalue_4 (Math|Conversions|ToFloat(Integer) _lod_4))
  (LocalVariables|SetLeftTimeStart (Class|SplineComponent|GetTimeatDistanceAlongSpline _splineleft_2 (Spline|GetDistanceAlongSplineatSplinePoint _splineleft_2 Index)))
  (LocalVariables|SetLeftTimeEnd (Class|SplineComponent|GetTimeatDistanceAlongSpline _splineleft_2 (Spline|GetDistanceAlongSplineatSplinePoint _splineleft_2 (+ Index 1))))
  (LocalVariables|SetRightTimeStart (Class|SplineComponent|GetTimeatDistanceAlongSpline _splineright_3 (Spline|GetDistanceAlongSplineatSplinePoint _splineright_3 Index)))
  (LocalVariables|SetRightTimeEnd (Class|SplineComponent|GetTimeatDistanceAlongSpline _splineright_3 (Spline|GetDistanceAlongSplineatSplinePoint _splineright_3 (+ Index 1))))
  (for _index (range 1 (Variables|Default|GetLOD))
    ;[1 1 1] Set Right Segment Start Time
    (LocalVariables|SetRightSegmentTimeStart (Math|Float|Lerp (LocalVariables|GetRightTimeStart) (LocalVariables|GetRightTimeEnd) (- (/ (Math|Conversions|ToFloat(Integer) _index) _returnvalue_4) (/ 1.0 _returnvalue_4))))
    ;[1 1 1] Set Right Segment End Time
    (LocalVariables|SetRightSegmentTimeEnd (Math|Float|Lerp (LocalVariables|GetRightTimeStart) (LocalVariables|GetRightTimeEnd) (- (/ (Math|Conversions|ToFloat(Integer) (+ _index 1)) _returnvalue_3) (/ 1.0 _returnvalue_3))))
    ;[1 1 1] Set Right Segment Start Time
    (LocalVariables|SetLeftSegmentTimeStart (Math|Float|Lerp (LocalVariables|GetLeftTimeStart) (LocalVariables|GetLeftTimeEnd) (- (/ (Math|Conversions|ToFloat(Integer) _index) _returnvalue_2) (/ 1.0 _returnvalue_2))))
    ;[1 1 1] Set Right Segment End Time
    (LocalVariables|SetLeftSegmentTimeEnd (Math|Float|Lerp (LocalVariables|GetLeftTimeStart) (LocalVariables|GetLeftTimeEnd) (- (/ (Math|Conversions|ToFloat(Integer) (+ _index 1)) _returnvalue) (/ 1.0 _returnvalue))))
    (bind _returnvalue_5 (AddComponent|AddSplineMeshComponent false))
    (SplineMesh|SetStartandEnd _returnvalue_5 (Spline|GetLocationatTime _splineright_2 (LocalVariables|GetRightSegmentTimeStart) "Local" false) (Math|Vector|GetVectorArrayAverage (Utilities|Array|MakeArray (Math|Vector|Normalize (Class|SplineComponent|GetTangentatTime _splineright_2 (LocalVariables|GetRightSegmentTimeStart) "Local" false)) (Math|Vector|Normalize (Class|SplineComponent|GetTangentatTime _splineleft_3 (LocalVariables|GetLeftSegmentTimeStart) "Local" false)))) (Spline|GetLocationatTime _splineright_2 (LocalVariables|GetRightSegmentTimeEnd) "Local" false) (Math|Vector|GetVectorArrayAverage (Utilities|Array|MakeArray (Math|Vector|Normalize (Class|SplineComponent|GetTangentatTime _splineright_2 (LocalVariables|GetRightSegmentTimeEnd) "Local" false)) (Math|Vector|Normalize (Class|SplineComponent|GetTangentatTime _splineleft_3 (LocalVariables|GetLeftSegmentTimeEnd) "Local" false)))) true :!class /Script/Engine.SplineMeshComponent)
    (bind _up (CallFunction|GetAxesfromTwoPoints (Spline|GetLocationatTime _splineright (LocalVariables|GetRightSegmentTimeStart) "Local" false) (Class|SplineComponent|GetTangentatTime _splineright (LocalVariables|GetRightSegmentTimeStart) "Local" false) (Spline|GetLocationatTime _splineleft (LocalVariables|GetLeftSegmentTimeStart) "Local" false) (Class|SplineComponent|GetTangentatTime _splineleft (LocalVariables|GetLeftSegmentTimeStart) "Local" false)))
    (bind _up_2 (CallFunction|GetAxesfromTwoPoints (Spline|GetLocationatTime _splineright (LocalVariables|GetRightSegmentTimeEnd) "Local" false) (Class|SplineComponent|GetTangentatTime _splineright (LocalVariables|GetRightSegmentTimeEnd) "Local" false) (Spline|GetLocationatTime _splineleft (LocalVariables|GetLeftSegmentTimeEnd) "Local" false) (Class|SplineComponent|GetTangentatTime _splineleft (LocalVariables|GetLeftSegmentTimeEnd) "Local" false)))
    (bind _midpoint (CallFunction|Midpoint _up _up_2))
    (SplineMesh|SetSplineUpDir _returnvalue_5 _midpoint true)
    (SplineMesh|SetStartScale _returnvalue_5 (Math|Vector2D|MakeVector2D (/ (Math|Vector|Distance(Vector) (Spline|GetLocationatTime _splineright (LocalVariables|GetRightSegmentTimeStart) "Local" false) (Spline|GetLocationatTime _splineleft (LocalVariables|GetLeftSegmentTimeStart) "Local" false)) 1e+03) 1.0) true :!class /Script/Engine.SplineMeshComponent)
    (SplineMesh|SetEndScale _returnvalue_5 (Math|Vector2D|MakeVector2D (/ (Math|Vector|Distance(Vector) (Spline|GetLocationatTime _splineright (LocalVariables|GetRightSegmentTimeEnd) "Local" false) (Spline|GetLocationatTime _splineleft (LocalVariables|GetLeftSegmentTimeEnd) "Local" false)) 1e+03) 1.0) true :!class /Script/Engine.SplineMeshComponent)
    (Transformation|AttachComponentToComponent _returnvalue_5 (Variables|Default|GetSplineLeft) "None" "KeepRelative" "KeepRelative" "KeepRelative" true)
    (AddComponent|AddArrowComponent false (Math|Transform|MakeTransform (Spline|GetLocationatTime _splineleft_3 (LocalVariables|GetLeftSegmentTimeStart) "Local" false) (Math|Conversions|RotationFromXVector (Math|Vector|Normalize (Class|SplineComponent|GetTangentatTime _splineleft_3 (LocalVariables|GetLeftSegmentTimeStart) "Local" false))) "1.000000,1.000000,1.000000"))
    (AddComponent|AddArrowComponent false (Math|Transform|MakeTransform (Spline|GetLocationatTime _splineleft_3 (LocalVariables|GetLeftSegmentTimeEnd) "Local" false) (Math|Conversions|RotationFromXVector (Math|Vector|Normalize (Class|SplineComponent|GetTangentatTime _splineleft_3 (LocalVariables|GetLeftSegmentTimeEnd) "Local" false))) "1.000000,1.000000,1.000000"))))

(fn CalculateRightatIndex
  (params (Index :type Integer))
  (return (- (.location (Spline|GetTransformatSplinePoint (Variables|Default|GetSplineLeft) Index "Local" false)) (.location (Spline|GetTransformatSplinePoint (Variables|Default|GetSplineRight) Index "Local" false)))))

(fn CheckAddDelete)

(fn GetUpatSplineIndex
  (params (Index :type Integer))
  (bind _splineleft (Variables|Default|GetSplineLeft))
  (bind (_location _tangent) (Spline|GetLocationandTangentatSplinePoint _splineleft Index "Local"))
  (return (Math|Vector|RotateVectorAroundAxis (- _location (.Location (Spline|GetLocationandTangentatSplinePoint (Variables|Default|GetSplineRight) Index "Local"))) -9e+01 _tangent)))

(fn GetMidpointatIndex
  (params (Index :type Integer))
  (bind _minpoints (Variables|Default|GetminPoints))
  ;[1 1 1] Bounds Checking
  (if (< Index 0)
    (LocalVariables|SetTargetIndex 0)
    (elif (> Index _minpoints)
      (LocalVariables|SetTargetIndex _minpoints)
      (else
        (LocalVariables|SetTargetIndex Index))))
  (return (/ (+ (.Location (Spline|GetLocationandTangentatSplinePoint (Variables|Default|GetSplineLeft) (LocalVariables|GetTargetIndex) "Local")) (.Location (Spline|GetLocationandTangentatSplinePoint (Variables|Default|GetSplineRight) (LocalVariables|GetTargetIndex) "Local"))) 2)))

(fn Midpoint
  (params (Vector1 :type Vector) (Vector2 :type Vector))
  (return (/ (+ Vector1 Vector2) 2)))

(fn GetForwardatIndex
  (params (Index :type Integer))
  (bind _midpoint (CallFunction|Midpoint (Spline|GetTangentatSplinePoint (Variables|Default|GetSplineLeft) Index "Local") (Spline|GetTangentatSplinePoint (Variables|Default|GetSplineRight) Index "Local")))
  (return _midpoint))

(fn GetUpatMeshIndex
  (params (Index :type Integer))
  (bind _up_vector (CallFunction|GetUpatSplineIndex Index))
  (bind _up_vector_2 (CallFunction|GetUpatSplineIndex (+ Index 1)))
  (bind _midpoint (CallFunction|Midpoint _up_vector_2 _up_vector))
  (return _midpoint))

(fn GetScaleatIndex
  (params (Index :type Integer))
  (return (/ (Math|Vector|Distance(Vector) (.Location (Spline|GetLocationandTangentatSplinePoint (Variables|Default|GetSplineLeft) Index "Local")) (.Location (Spline|GetLocationandTangentatSplinePoint (Variables|Default|GetSplineRight) Index "Local"))) 1e+03)))

(fn GetAxesfromTwoPoints
  (params (RightPosition :type Vector) (RightTangent :type Vector) (LeftLocation :type Vector) (LeftTangent :type Vector))
  (bind _midpoint (CallFunction|Midpoint RightTangent LeftTangent))
  (return _midpoint (- LeftLocation RightPosition) (Math|Vector|RotateVectorAroundAxis (- LeftLocation RightPosition) -9e+01 LeftTangent)))