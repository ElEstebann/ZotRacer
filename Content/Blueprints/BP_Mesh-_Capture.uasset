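; BP_Mesh-_Capture renders its own configurable mesh into a render target as a rotating view.
; The construction script applies the mesh, scale and materials to the Cube component.
; BeginPlay limits the scene capture to this actor, then attaches it to a focus component, setting distance, pitch and vertical offset.
; Tick yaws that focus component a fixed step per frame, orbiting the capture independently of delta time.
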(event EventBeginPlay
  (bind _scenecapturecomponent2d (Variables|Default|GetSceneCaptureComponent2D))
  (bind _scenecapturecomponent2d_2 (Variables|Default|GetSceneCaptureComponent2D))
  (Rendering|SceneCapture|ClearShowOnlyComponents _scenecapturecomponent2d)
  (Rendering|SceneCapture|ShowOnlyActorComponents _scenecapturecomponent2d self true)
  (Variables|/Script/Engine.SceneCaptureComponent2D|SetTextureTarget (Variables|Default|GetSceneCaptureComponent2D) (Variables|Default|GetRenderTarget))
  (bind _output_get (Variables|Default|SetFocusMesh (Variables|Default|GetFocus)))
  (Variables|Default|SetAxis (Math|Vector|GetUpVector _output_get))
  (Transformation|AttachComponentToComponent _scenecapturecomponent2d_2 _output_get "None" "SnapToTarget" "KeepRelative" "KeepRelative" true)
  (Transformation|SetRelativeLocation _scenecapturecomponent2d_2 (- (.location (Transformation|GetRelativeTransform _scenecapturecomponent2d_2)) (Math|Vector|MakeVector (Variables|Default|GetDistance) 0.0 0.0)) false false)
  (Transformation|AddRelativeRotation (Variables|Default|GetFocusMesh) (Math|Rotator|MakeRotator 0.0 (* (Variables|Default|GetAngle) -1.0) 0.0) false false)
  (Transformation|SetRelativeLocation (Variables|Default|GetFocusMesh) (+ (Variables|/Script/Engine.SceneComponent|GetRelativeLocation (Variables|Default|GetFocusMesh)) (Math|Vector|MakeVector 0.0 0.0 (Variables|Default|GetVerticalOffset))) false false))

(event Collision|EventActorBeginOverlap
  (params (OtherActor :type Actor%20Object%20Reference)))

(event EventTick
  (params (DeltaSeconds :type Float%20%28single-precision%29))
  (Transformation|AddRelativeRotation (Variables|Default|GetFocusMesh) "0.000000,1.000000,0.000000" false false))

(fn ConstructionScript
  (bind _cube (Variables|Default|GetCube))
  (Components|StaticMesh|SetStaticMesh _cube (Variables|Default|GetMesh))
  (Transformation|SetRelativeScale3D _cube (Variables|Default|GetMeshScale))
  (for (_array_element _array_index) (Variables|Default|GetMaterials)
    (Rendering|Material|SetMaterial _cube _array_index _array_element)))