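; BP_Racecar is a physics-driven racecar prototype controlled with A, D and Space.
; Each Tick pushes the Cube along GravityVector's forward axis for custom gravity, plus along AccelerationVector's while Space is held.
; A and D apply opposite roll offsets to the Sphere on press and undo them on release.
; Tick also prints speed from the Cube's frame-to-frame displacement; HandleRotation is an empty stub.
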(event EventBeginPlay
  (Variables|Default|SetLastLocation (Transformation|GetWorldLocation (Variables|Default|GetCube))))

(event Collision|EventActorBeginOverlap
  (params (OtherActor :type Actor%20Object%20Reference)))

(event EventTick
  (params (DeltaSeconds :type Float%20%28single-precision%29))
  (CallFunction|HandleGravity)
  (CallFunction|HandleAcceleration)
  (CallFunction|GetSpeed))

(event Input|KeyboardEvents|SpaceBar
  (params (Key :type Key%20Structure :default "None"))
  (:Pressed
    (Variables|Default|SetAccelerating true))
  (:Released
    (Variables|Default|SetAccelerating false)))

(event Input|KeyboardEvents|A
  (params (Key :type Key%20Structure :default "None"))
  (bind _sphere (Variables|Default|GetSphere))
  (bind _delta_rotation_x__roll_ (Variables|Default|GetDelta%20Rotation%20X%20%28Roll%29))
  (:Pressed
    (Transformation|AddLocalRotation _sphere (Math|Rotator|MakeRotator (* _delta_rotation_x__roll_ -1.0) 0.0 0.0) false false))
  (:Released
    (Transformation|AddLocalRotation _sphere (Math|Rotator|MakeRotator _delta_rotation_x__roll_ 0.0 0.0) false false)))

(event Input|KeyboardEvents|D
  (params (Key :type Key%20Structure :default "None"))
  (bind _sphere (Variables|Default|GetSphere))
  (bind _delta_rotation_x__roll_ (Variables|Default|GetDelta%20Rotation%20X%20%28Roll%29))
  (:Pressed
    (Transformation|AddLocalRotation _sphere (Math|Rotator|MakeRotator _delta_rotation_x__roll_ 0.0 0.0) false false))
  (:Released
    (Transformation|AddLocalRotation _sphere (Math|Rotator|MakeRotator (* _delta_rotation_x__roll_ -1.0) 0.0 0.0) false false)))

(fn ConstructionScript)

(fn HandleGravity
  (Physics|AddForce (Variables|Default|GetCube) (* (Math|Vector|GetForwardVector (Variables|Default|GetGravityVector)) 5e+05) "None" false))

(fn HandleRotation)

(fn HandleAcceleration
  (if (Variables|Default|GetAccelerating)
    (Physics|AddForce (Variables|Default|GetCube) (* (Math|Vector|GetForwardVector (Variables|Default|GetAccelerationVector)) 5e+06) "None" false)))

(fn GetSpeed
  (bind _cube (Variables|Default|GetCube))
  (bind _returnvalue (Transformation|GetWorldLocation _cube))
  (Development|PrintString (Utilities|String|ToString(Float) (/ (Math|Vector|Distance(Vector) (Variables|Default|GetLastLocation) _returnvalue) (Utilities|Time|GetWorldDeltaSeconds))))
  (Variables|Default|SetLastLocation _returnvalue))