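; Road actor that builds spline mesh segments from a left and right edge spline in the construction script.
; Segments start and end on the right spline, use averaged tangents and scale width by the distance between edges.
; Banking comes from axes derived from both edges, with each roll step clamped against the previous to accumulate continuously.
; Arrow components visualize the vectors; point add/delete detection is unwired.
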(event EventBeginPlay)

(event Collision|EventActorBeginOverlap
  (params (OtherActor :type Actor%20Object%20Reference)))

(event EventTick
  (params (DeltaSeconds :type Float%20%28single-precision%29)))

(fn ConstructionScript
  ;[1 1 1] Initialization
  (CallFunction|InitializeSplines)
  (CallFunction|InitializeArrays)
  (CallFunction|DrawDebug)
  (for _index (range 0 (- (Variables|Default|GetminPoints) 2))
    (CallFunction|SetMeshatSplineIndex _index)))

(fn DrawDebug
  (bind _splineright (Variables|Default|GetSplineRight))
  (bind _returnvalue (Spline|GetNumberOfSplinePoints _splineright))
  (bind _returnvalue_2 (- _returnvalue 1))
  ;[1 1 1] Comment
  (for _index (range 0 _returnvalue_2)
    (bind _up_vector (CallFunction|GetUpatSplineIndex _index))
    (AddComponent|AddArrowComponent false (Math|Transform|MakeTransform "0, 0, 0" (Math|Conversions|RotationFromXVector _up_vector) "1.000000,1.000000,1.000000"))
    (bind _right_axis (CallFunction|CalculateRightatIndex _index))
    (AddComponent|AddArrowComponent false (Math|Transform|MakeTransform "0, 0, 0" (Math|Conversions|RotationFromXVector _right_axis) "1.000000,1.000000,1.000000"))
    ;[1 1 1] Comment
    (bind _newparam (CallFunction|GetMidpointatIndex (+ (stale _index_2) 1)))
    (bind _newparam_2 (CallFunction|GetMidpointatIndex (stale _index_2)))
    (bind _midpoint (CallFunction|Midpoint _newparam_2 _newparam))
    (bind _up_vector_2 (CallFunction|GetUpatMeshIndex (stale _index_2)))
    (AddComponent|AddArrowComponent false (Math|Transform|MakeTransform _midpoint (Math|Conversions|RotationFromXVector _up_vector_2) "1.000000,1.000000,1.000000")))
  (for _index_2 (range 0 (- _returnvalue_2 1)) ; Iterate through each mesh index
    (bind _newparam_3 (CallFunction|GetMidpointatIndex (+ _index_2 1)))
    (bind _newparam_4 (CallFunction|GetMidpointatIndex _index_2))
    (bind _midpoint_2 (CallFunction|Midpoint _newparam_4 _newparam_3))
    (bind _up_vector_3 (CallFunction|GetUpatMeshIndex _index_2))
    (AddComponent|AddArrowComponent false (Math|Transform|MakeTransform _midpoint_2 (Math|Conversions|RotationFromXVector _up_vector_3) "1.000000,1.000000,1.000000"))))

(fn InitializeArrays
  (bind _minpoints (Variables|Default|GetminPoints))
  (bind _rolllist (Variables|Default|GetrollList))
  (bind _rolllist_2 (Variables|Default|GetrollList))
  (bind _returnvalue (- _minpoints 1))
  (Utilities|Array|Resize (Variables|Default|GetmeshList) _returnvalue)
  (Utilities|Array|Resize _rolllist _minpoints)
  (Utilities|Array|SetArrayElem _rolllist 0 0.0)
  (for _index (range 1 _returnvalue)
    (bind _up_vector (CallFunction|GetUpatSplineIndex _index))
    (bind _right_axis (CallFunction|CalculateRightatIndex _index))
    (bind _forward_vector (CallFunction|GetForwardatIndex _index))
    (Utilities|Array|SetArrayElem _rolllist_2 _index (+ (Math|Trig|DegreesToRadians (Math|Float|ClampAngle (Math|Trig|RadiansToDegrees (- (- (* (Math|Trig|DegreesToRadians (.roll (Math|Rotator|MakeRotationfromAxes _forward_vector _right_axis _up_vector))) -1.0) 3.14) (Utilities|Array|Get(acopy) _rolllist_2 (- _index 1)))) -9e+01 9e+01)) (Utilities|Array|Get(acopy) _rolllist_2 (- _index 1))))))

(fn InitializeSplines
  (bind _output_get (Variables|Default|SetminPoints (Math|Integer|Min(Integer) (Spline|GetNumberOfSplinePoints (Variables|Default|GetSplineRight)) (Spline|GetNumberOfSplinePoints (Variables|Default|GetSplineLeft)))))
  (for _index (range 0 (- _output_get 1))
    _))

(fn SetMeshatSplineIndex
  (params (Index :type Integer))
  (bind _returnvalue (+ Index 1))
  (bind _rolllist (Variables|Default|GetrollList))
  (bind _splineleft (Variables|Default|GetSplineLeft))
  (bind _splineright (Variables|Default|GetSplineRight))
  (bind _splineleft_2 (Variables|Default|GetSplineLeft))
  (bind _splineright_2 (Variables|Default|GetSplineRight))
  (bind (_location _tangent) (Spline|GetLocationandTangentatSplinePoint _splineleft_2 Index "Local"))
  (bind (_location_2 _tangent_2) (Spline|GetLocationandTangentatSplinePoint _splineright_2 Index "Local"))
  (bind (_location_3 _tangent_3) (Spline|GetLocationandTangentatSplinePoint _splineleft _returnvalue "Local"))
  (bind (_location_4 _tangent_4) (Spline|GetLocationandTangentatSplinePoint _splineright _returnvalue "Local"))
  (bind _returnvalue_2 (AddComponent|AddSplineMeshComponent false (Math|Transform|MakeTransform (Math|Vector|MakeVector 0.0 0.0 (Variables|Default|GetSplineEditOffset)) "0, 0, 0" "1.000000,1.000000,1.000000")))
  (CallFunction|Midpoint _location _location_2)
  (bind _midpoint (CallFunction|Midpoint _tangent _tangent_2))
  (CallFunction|Midpoint _location_3 _location_4)
  (bind _midpoint_2 (CallFunction|Midpoint _tangent_3 _tangent_4))
  (SplineMesh|SetStartandEnd _returnvalue_2 _location_2 _midpoint _location_4 _midpoint_2 true :!class /Script/Engine.SplineMeshComponent)
  ;[1 1 1] Set Start & End Scales relative to point distances
  (bind _scale (CallFunction|GetScaleatIndex Index))
  (SplineMesh|SetStartScale _returnvalue_2 (Math|Vector2D|MakeVector2D _scale 1.0) true :!class /Script/Engine.SplineMeshComponent)
  (bind _scale_2 (CallFunction|GetScaleatIndex (+ Index 1)))
  (SplineMesh|SetEndScale _returnvalue_2 (Math|Vector2D|MakeVector2D _scale_2 1.0) true :!class /Script/Engine.SplineMeshComponent)
  ;[1 1 1] Set Rolls For Start and End
  (Class|SplineMeshComponent|SetStartRoll _returnvalue_2 (Utilities|Array|Get(acopy) _rolllist Index) true)
  (Class|SplineMeshComponent|SetEndRoll _returnvalue_2 (Utilities|Array|Get(acopy) _rolllist (+ Index 1)) true)
  ;[1 1 1] Add Mesh to parent spline
  (Transformation|AttachComponentToComponent _returnvalue_2 (Variables|Default|GetSplineRight) "None" "KeepRelative" "KeepRelative" "KeepRelative" true))

(fn CalculateRightatIndex
  (params (Index :type Integer))
  (return (- (.location (Spline|GetTransformatSplinePoint (Variables|Default|GetSplineLeft) Index "Local" false)) (.location (Spline|GetTransformatSplinePoint (Variables|Default|GetSplineRight) Index "Local" false)))))

(fn CheckAddDelete)

(fn GetUpatSplineIndex
  (params (Index :type Integer))
  (bind _splineleft (Variables|Default|GetSplineLeft))
  (bind (_location _tangent) (Spline|GetLocationandTangentatSplinePoint _splineleft Index "Local"))
  (return (Math|Vector|RotateVectorAroundAxis (- _location (.Location (Spline|GetLocationandTangentatSplinePoint (Variables|Default|GetSplineRight) Index "Local"))) -9e+01 _tangent)))

(fn GetMidpointatIndex
  (params (Index :type Integer))
  (bind _minpoints (Variables|Default|GetminPoints))
  ;[1 1 1] Bounds Checking
  (if (< Index 0)
    (LocalVariables|SetTargetIndex 0)
    (elif (> Index _minpoints)
      (LocalVariables|SetTargetIndex _minpoints)
      (else
        (LocalVariables|SetTargetIndex Index))))
  (return (/ (+ (.Location (Spline|GetLocationandTangentatSplinePoint (Variables|Default|GetSplineLeft) (LocalVariables|GetTargetIndex) "Local")) (.Location (Spline|GetLocationandTangentatSplinePoint (Variables|Default|GetSplineRight) (LocalVariables|GetTargetIndex) "Local"))) 2)))

(fn Midpoint
  (params (Vector1 :type Vector) (Vector2 :type Vector))
  (return (/ (+ Vector1 Vector2) 2)))

(fn GetForwardatIndex
  (params (Index :type Integer))
  (bind _midpoint (CallFunction|Midpoint (Spline|GetTangentatSplinePoint (Variables|Default|GetSplineLeft) Index "Local") (Spline|GetTangentatSplinePoint (Variables|Default|GetSplineRight) Index "Local")))
  (return _midpoint))

(fn GetUpatMeshIndex
  (params (Index :type Integer))
  (bind _up_vector (CallFunction|GetUpatSplineIndex Index))
  (bind _up_vector_2 (CallFunction|GetUpatSplineIndex (+ Index 1)))
  (bind _midpoint (CallFunction|Midpoint _up_vector_2 _up_vector))
  (return _midpoint))

(fn GetScaleatIndex
  (params (Index :type Integer))
  (return (/ (Math|Vector|Distance(Vector) (.Location (Spline|GetLocationandTangentatSplinePoint (Variables|Default|GetSplineLeft) Index "Local")) (.Location (Spline|GetLocationandTangentatSplinePoint (Variables|Default|GetSplineRight) Index "Local"))) 1e+03)))