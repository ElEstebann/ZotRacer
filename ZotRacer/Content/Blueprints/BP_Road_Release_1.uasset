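; Spline road actor that builds spline mesh components along its spline in the construction script.
; Each segment is split into LOD pieces by CreateMeshFromDistances, with scaled-down tangents, eased roll and spline scale.
; Per-segment meshes carry forward when unset, and flip points toggle a persistent 180-degree roll.
; MapViewMode forces one piece per segment without assigning meshes, and DebugLines draws arrow components along the spline.
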(event EventBeginPlay)

(event Collision|EventActorBeginOverlap
  (params (OtherActor :type Actor%20Object%20Reference)))

(event EventTick
  (params (DeltaSeconds :type Float%20%28single-precision%29)))

(fn ConstructionScript
  (bind _spline (Variables|Default|GetSpline))
  (bind _spline_2 (Variables|Default|GetSpline))
  (bind _spline_3 (Variables|Default|GetSpline))
  (bind _easefunction (Variables|Default|GetEaseFunction))
  (if (Variables|Default|GetMapViewMode)
    (Variables|Default|SetLOD 1))
  (LocalVariables|SetCurrentMesh (Utilities|Array|Get(acopy) (Variables|Default|GetMeshes)))
  (for _index (range 0 (- (Class|SplineComponent|GetNumberOfSplineSegments _spline) 1)) ; Iterate over every spline segment
    (LocalVariables|SetStartDisrance (Spline|GetDistanceAlongSplineatSplinePoint _spline _index))
    (LocalVariables|SetEndDistance (Spline|GetDistanceAlongSplineatSplinePoint _spline (+ _index 1)))
    ;[1 1 1] Check If Flip Point Set
    (if (Utilities|Array|Get(acopy) (Variables|Default|GetFlip%20Points) _index)
      (LocalVariables|SetFlipping (not (LocalVariables|GetFlipping))))
    (if (Utilities|IsValid (Utilities|Array|Get(acopy) (Variables|Default|GetMeshes) _index))
      (Variables|Default|SetCurrent%20Mesh (Utilities|Array|Get(acopy) (Variables|Default|GetMeshes) _index)))
    (for _index_2 (range 1 (Variables|Default|GetLOD))
      (CallFunction|CreateMeshfromDistances (Math|Float|Lerp (LocalVariables|GetStartDisrance) (LocalVariables|GetEndDistance) (- (/ (Math|Conversions|ToFloat(Integer) _index_2) (Math|Conversions|ToFloat(Integer) (Variables|Default|GetLOD))) (/ 1.0 (Math|Conversions|ToFloat(Integer) (Variables|Default|GetLOD))))) (Math|Float|Lerp (LocalVariables|GetStartDisrance) (LocalVariables|GetEndDistance) (- (/ (Math|Conversions|ToFloat(Integer) (+ _index_2 1)) (Math|Conversions|ToFloat(Integer) (Variables|Default|GetLOD))) (/ 1.0 (Math|Conversions|ToFloat(Integer) (Variables|Default|GetLOD))))) (LocalVariables|GetFlipping) (Variables|Default|GetCurrent%20Mesh) (Math|Interpolation|Ease _easefunction (- (/ (Math|Conversions|ToFloat(Integer) _index_2) (Math|Conversions|ToFloat(Integer) (Variables|Default|GetLOD))) (/ 1.0 (Math|Conversions|ToFloat(Integer) (Variables|Default|GetLOD)))) (Spline|GetRollatSplinePoint _spline_3 _index "Local") (Spline|GetRollatSplinePoint _spline_3 (+ _index 1) "Local") 2.0) (Math|Interpolation|Ease _easefunction (- (/ (Math|Conversions|ToFloat(Integer) (+ _index_2 1)) (Math|Conversions|ToFloat(Integer) (Variables|Default|GetLOD))) (/ 1.0 (Math|Conversions|ToFloat(Integer) (Variables|Default|GetLOD)))) (Spline|GetRollatSplinePoint _spline_2 _index "Local") (Spline|GetRollatSplinePoint _spline_2 (+ _index 1) "Local") 2.0))))
  (CallFunction|DrawDebug))

(fn InitializeArrays
  (bind _spline (Variables|Default|GetSpline))
  (bind _returnvalue (Class|SplineComponent|GetNumberOfSplineSegments _spline))
  (Utilities|Array|Resize (Variables|Default|GetMeshes) _returnvalue)
  (Utilities|Array|Resize (Variables|Default|GetFlip%20Points) (+ _returnvalue 1)))

(fn DrawDebug
  (bind _spline (Variables|Default|GetSpline))
  (bind _returnvalue (Class|SplineComponent|GetNumberOfSplineSegments _spline))
  (if (Variables|Default|GetDebugLines)
    (for _index (range 1 (- (* _returnvalue 10) 1))
      (AddComponent|AddArrowComponent false (Math|Transform|MakeTransform (Spline|GetLocationatDistanceAlongSpline _spline (Math|Float|Lerp 1.0 (Spline|GetSplineLength _spline) (/ (Math|Conversions|ToFloat(Integer) _index) (Math|Conversions|ToFloat(Integer) (Math|Conversions|ToFloat(Integer) (* _returnvalue 10))))) "Local") (Math|Conversions|RotationFromXVector (Class|SplineComponent|GetUpVectoratDistanceAlongSpline _spline (Math|Float|Lerp 1.0 (Spline|GetSplineLength _spline) (/ (Math|Conversions|ToFloat(Integer) _index) (Math|Conversions|ToFloat(Integer) (Math|Conversions|ToFloat(Integer) (* _returnvalue 10))))) "Local")) "1.000000,1.000000,1.000000"))
      (AddComponent|AddArrowComponent false (Math|Transform|MakeTransform (Spline|GetLocationatDistanceAlongSpline _spline (Math|Float|Lerp 1.0 (Spline|GetSplineLength _spline) (/ (Math|Conversions|ToFloat(Integer) _index) (Math|Conversions|ToFloat(Integer) (Math|Conversions|ToFloat(Integer) (* _returnvalue 10))))) "Local") (Spline|GetRotationatDistanceAlongSpline _spline 0.0 "Local") "1.000000,1.000000,1.000000")))))

(fn CreateMeshfromDistances
  (params (StartDistance :type Float%20%28double-precision%29) (EndDistance :type Float%20%28double-precision%29) (Flipped :type Boolean) (Mesh :type Static%20Mesh%20Object%20Reference) (StartRoll :type Float%20%28double-precision%29) (EndRoll :type Float%20%28double-precision%29))
  (bind _lod (Variables|Default|GetLOD))
  (bind _spline (Variables|Default|GetSpline))
  (bind _spline_2 (Variables|Default|GetSpline))
  (bind _spline_3 (Variables|Default|GetSpline))
  (bind _returnvalue (Spline|GetLocationatDistanceAlongSpline _spline_3 EndDistance "Local"))
  (bind _returnvalue_2 (Spline|GetTangentatDistanceAlongSpline _spline_3 EndDistance "Local"))
  (bind _returnvalue_3 (Spline|GetLocationatDistanceAlongSpline _spline_3 StartDistance "Local"))
  (bind _returnvalue_4 (Spline|GetTangentatDistanceAlongSpline _spline_3 StartDistance "Local"))
  (bind _returnvalue_5 (Class|SplineComponent|GetScaleatDistanceAlongSpline _spline_2 StartDistance))
  (bind _returnvalue_6 (Class|SplineComponent|GetScaleatDistanceAlongSpline _spline_2 EndDistance))
  (bind _returnvalue_7 (AddComponent|AddSplineMeshComponent true))
  (if (Variables|Default|GetDebugLines)
    (AddComponent|AddArrowComponent false (Math|Transform|MakeTransform _returnvalue_3 (Math|Conversions|RotationFromXVector _returnvalue_4) "1.000000,1.000000,1.000000"))
    (AddComponent|AddArrowComponent false (Math|Transform|MakeTransform _returnvalue (Math|Conversions|RotationFromXVector _returnvalue_2) "1.000000,1.000000,1.000000")))
  (if (> (Variables|Default|GetLOD) 1)
    (SplineMesh|SetStartandEnd _returnvalue_7 _returnvalue_3 (/ _returnvalue_4 _lod) _returnvalue (/ _returnvalue_2 _lod) true :!class /Script/Engine.SplineMeshComponent)
    (else
      (SplineMesh|SetStartandEnd _returnvalue_7 _returnvalue_3 _returnvalue_4 _returnvalue _returnvalue_2 true :!class /Script/Engine.SplineMeshComponent)))
  ;[1 1 1] Set Roll
  (LocalVariables|SetRoll%20Offset 0.0)
  (if Flipped
    (LocalVariables|SetRoll%20Offset 1.8e+02))
  (Class|SplineMeshComponent|SetStartRoll _returnvalue_7 (Math|Trig|DegreesToRadians (+ (LocalVariables|GetRoll%20Offset) StartRoll)) true)
  (if (Variables|Default|GetDebugLines)
    (AddComponent|AddArrowComponent false (Math|Transform|MakeTransform (Spline|GetLocationatDistanceAlongSpline _spline StartDistance "Local") (Math|Conversions|RotationFromXVector (Class|SplineComponent|GetUpVectoratDistanceAlongSpline _spline StartDistance "Local")) "1.000000,1.000000,1.000000")))
  (Class|SplineMeshComponent|SetEndRoll _returnvalue_7 (Math|Trig|DegreesToRadians (+ (LocalVariables|GetRoll%20Offset) EndRoll)) true)
  ;[1 1 1] Set Scale
  (SplineMesh|SetStartScale _returnvalue_7 (Math|Vector2D|MakeVector2D (.y _returnvalue_5) (.z _returnvalue_5)) true :!class /Script/Engine.SplineMeshComponent)
  (SplineMesh|SetEndScale _returnvalue_7 (Math|Vector2D|MakeVector2D (.y _returnvalue_6) (.z _returnvalue_6)) true :!class /Script/Engine.SplineMeshComponent)
  ;[1 1 1] Set Static Mesh
  (if (Variables|Default|GetMapViewMode)
    _
    (else
      (Components|StaticMesh|SetStaticMesh _returnvalue_7 Mesh)
      (Class|PrimitiveComponent|SetUseCCD _returnvalue_7 false "None")))
  (Transformation|AttachComponentToComponent _returnvalue_7 (Variables|Default|GetSpline) "None" "KeepRelative" "KeepRelative" "KeepRelative" true))