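; Child of a Mobius strip Blueprint that animates its StaticMesh in an endless loop along the Path spline.
; Each Tick runs the parent logic, accumulates elapsed time and wraps it by the spline time at full length.
; That time samples local location and rotation without constant velocity, applying both to the mesh with a yaw offset of minus 90 degrees.
; The construction script only calls the parent's.
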(event EventBeginPlay
  (|CallParentFunction) ; This node is disabled and will not be called.\nDrag off pins to build functionality.
)

(event Collision|EventActorBeginOverlap
  (params (OtherActor :type Actor%20Object%20Reference))
  (|CallParentFunction OtherActor) ; This node is disabled and will not be called.\nDrag off pins to build functionality.
)

(event EventTick
  (params (DeltaSeconds :type Float%20%28single-precision%29))
  (bind _path (Variables|Default|GetPath))
  (|CallParentFunction DeltaSeconds)
  (bind _output_get (Variables|Default|SetTimeElapsed (+ (Utilities|Time|GetWorldDeltaSeconds) (Variables|Default|GetTimeElapsed))))
  (Transformation|SetRelativeLocationAndRotation (Variables|Default|GetStaticMesh) (Spline|GetLocationatTime _path (Math|Float|%(Float) _output_get (Class|SplineComponent|GetTimeatDistanceAlongSpline _path (Spline|GetSplineLength _path))) "Local" false) (Math|Rotator|MakeRotator (.roll (Class|SplineComponent|GetRotationatTime _path (Math|Float|%(Float) _output_get (Class|SplineComponent|GetTimeatDistanceAlongSpline _path (Spline|GetSplineLength _path))) "Local" false)) (.pitch (Class|SplineComponent|GetRotationatTime _path (Math|Float|%(Float) _output_get (Class|SplineComponent|GetTimeatDistanceAlongSpline _path (Spline|GetSplineLength _path))) "Local" false)) (+ (.yaw (Class|SplineComponent|GetRotationatTime _path (Math|Float|%(Float) _output_get (Class|SplineComponent|GetTimeatDistanceAlongSpline _path (Spline|GetSplineLength _path))) "Local" false)) -9e+01)) false false))

(fn ConstructionScript
  (|CallParentFunction))